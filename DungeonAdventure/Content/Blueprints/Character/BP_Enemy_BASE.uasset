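; BP_Enemy_BASE is a base enemy Blueprint that can walk in a given direction and hurts the hero on contact.
; WalkTowards feeds a world direction into movement input unless the BPCHealth component reports the enemy as defeated.
; When its HurtBox begins overlapping the HurtBox of a BP_Hero, it applies fixed damage to that hero, with no defeated check on this path.
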(event `WalkTowards`
  (params (WorldDirection :type "Vector Structure"))
  (if (not (`/Game/Blueprints/Components/BPC_Health.IsDefeated` (`self.BPC_Health`)))
    (`self.AddMovementInput` WorldDirection)))

(event `self.HurtBox.OnComponentBeginOverlap`
  (params (OverlappedComponent :type "PrimitiveComponent Object Reference") (OtherActor :type "Actor Object Reference") (OtherComp :type "PrimitiveComponent Object Reference") (OtherBodyIndex :type Integer) (bFromSweep :type Boolean) (SweepResult :type "HitResult Structure (by ref)"))
  (bind _asbp_hero (cast `/Game/Blueprints/Character/Hero/BP_Hero` OtherActor))
  (if (== (`/Game/Blueprints/Character/BP_DungeonChar_BASE.HurtBox` _asbp_hero) OtherComp)
    (`GameplayStatics.ApplyDamage` _asbp_hero 1.0 null self)))

(fn `UserConstructionScript`
  (`parent.UserConstructionScript`))